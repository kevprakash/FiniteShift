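; LevelGoal is a level-exit actor that ends the level when the player character overlaps it.
; The first PlayerCharacter overlap passes a DoOnce, calls StartWin on that character and plays a timeline that animates the goal's scale.
; When the timeline finishes, it opens the level named by the NextLevel variable.
; A local rotation node remains in the graph but is unconnected.
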(event EventBeginPlay)

(event Collision|EventActorBeginOverlap
  (params (OtherActor :type Actor%20Object%20Reference))
  (bind _asplayer_character (Utilities|Casting|CastToPlayerCharacter OtherActor))
  (Utilities|FlowControl|DoOnce false
    (:Completed
      (Default|StartWin _asplayer_character)
      (bind _actor_scale (Timeline|Timeline_0 PlayFromStart)
        (:Update
          (Transformation|SetActorScale3D (Math|Conversions|ToVector(Float) _actor_scale)))
        (:Finished
          (Game|OpenLevel(byName) (Variables|Default|GetNextLevel)))))))

(event EventTick
  (params (DeltaSeconds :type Float%20%28single-precision%29)))

(fn ConstructionScript)
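; JumpReset is a gem pickup that restores the player's air dash or air jump on overlap, depending on its Dash flag.
; The construction script picks the matching dash or jump sprite, and Tick bobs the Sphere on a sine wave.
; Collection disables collision and hides the sprite rather than removing the actor, so the Reset event can restore it, though nothing here calls Reset.
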(event Custom|Reset
  (Collision|SetCollisionEnabled (Variables|Default|GetSphere) "QueryOnly")
  (Rendering|SetVisibility (Variables|Default|GetPaperSprite) true false))

(event Custom|Destroy
  (Collision|SetCollisionEnabled (Variables|Default|GetSphere) "NoCollision")
  (Rendering|SetVisibility (Variables|Default|GetPaperSprite) false false))

(event EventTick
  (params (DeltaSeconds :type Float%20%28single-precision%29))
  (Transformation|SetRelativeLocation (Variables|Default|GetSphere) (Math|Vector|MakeVector 0.0 0.0 (* (Math|Trig|Sin(Degrees) (* (Utilities|Time|GetTimeSeconds) 1.8e+02)) 1e+01)) false false))

(event Collision|EventActorBeginOverlap
  (params (OtherActor :type Actor%20Object%20Reference))
  (bind _asplayer_character (Utilities|Casting|CastToPlayerCharacter OtherActor))
  (if (Variables|Default|GetbDash)
    (Variables|/Game/Blueprints/PlayerCharacter.PlayerCharacter_C|SetbCanAirDash _asplayer_character true)
    (else
      (Variables|/Game/Blueprints/PlayerCharacter.PlayerCharacter_C|SetbCanAirJump _asplayer_character true)))
  (CallFunction|Destroy))

(fn ConstructionScript
  (bind _papersprite (Variables|Default|GetPaperSprite))
  (if (Variables|Default|GetbDash)
    (Rendering|Components|Sprite|SetSprite _papersprite "/Game/Art/Sprites/DashGem_Sprite.DashGem_Sprite")
    (else
      (Rendering|Components|Sprite|SetSprite _papersprite "/Game/Art/Sprites/JumpGem_Sprite.JumpGem_Sprite"))))
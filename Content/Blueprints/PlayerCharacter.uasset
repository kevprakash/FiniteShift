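; Side-view platformer player character with a limited budget of jumps and dashes, shown on a counter widget component.
; Timeline-driven jump and dash fire velocity-change impulses, gated by counters, air-use flags and coyote time.
; Spending both budgets starts a self-destruct timer that StartWin cancels; Die refills counters and glides the character back to spawn with collision off.
; Tick eases the spring arm toward a signed-square-root velocity lead.
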(event Custom|Custom%20Jump
  (Math|Integer|DecrementInt (Variables|Default|GetJump%20Counter)
    (:%20%20
      (Variables|Default|SetbCanAirJump (or (not (AI|Components|NavMovement|IsFalling (Variables|Character|GetCharacterMovement))) (Variables|Default|GetCoyoteTimeActive)))
      (Physics|AddImpulse (Variables|Character|GetCharacterMovement) (- (* "0, 0,1.000000" (Variables|Default|GetJump%20Velocity)) (Math|Vector|MakeVector 0.0 0.0 (.Z (Math|Vector|BreakVector (Transformation|GetVelocity))))) true)
      (CallFunction|CheckifOutOfMovement))))

(event Custom|Dash
  (bind _charactermovement (Variables|Character|GetCharacterMovement))
  (Math|Integer|DecrementInt (Variables|Default|GetDash%20Counter)
    (:%20%20
      (Variables|Default|SetbCanAirDash (or (not (AI|Components|NavMovement|IsFalling (Variables|Character|GetCharacterMovement))) (Variables|Default|GetCoyoteTimeActive)))
      (Components|Movement|StopMovementImmediately _charactermovement)
      (Physics|AddImpulse _charactermovement (+ (* (Math|Vector|GetRightVector (Variables|Default|GetCamera)) (* (Math|Float|Sign(Float) (Input|AxisValues|GetLateral)) (Variables|Default|GetDash%20Velocity))) "0, 0,1.000000") true)
      (CallFunction|CheckifOutOfMovement))))

(event Custom|Die
  (bind _charactermovement (Variables|Character|GetCharacterMovement))
  (Variables|Default|SetbDashing false)
  (Variables|Default|SetbSelfDestruct false)
  (Utilities|Time|ClearandInvalidateTimerbyHandle (Variables|Default|GetSelfDestructTimer))
  (Variables|Default|SetbDead true)
  (Collision|SetCollisionEnabled (Variables|Default|GetCapsuleComponent) "NoCollision")
  (Variables|/Script/Engine.CharacterMovementComponent|SetGravityScale _charactermovement 0.0)
  (Components|Movement|StopMovementImmediately _charactermovement)
  (Input|DisableInput (Game|GetPlayerController 0))
  (CallFunction|ResetCounters)
  (bind _lerp_alpha (Timeline|Timeline_0 PlayFromStart)
    (:Update
      (Transformation|SetActorLocation (Math|Vector|Lerp(Vector) (Transformation|GetActorLocation) (Variables|Default|GetSpawn%20Location) _lerp_alpha) false false))
    (:Finished
      (Collision|SetCollisionEnabled (Variables|Default|GetCapsuleComponent) "QueryAndPhysics")
      (Variables|/Script/Engine.CharacterMovementComponent|SetGravityScale (Variables|Character|GetCharacterMovement) 1.0)
      (Input|EnableInput (Game|GetPlayerController 0)))
    (:Mark%20Undead
      (Variables|Default|SetbDead false))))

(event Custom|Reset%20Counters
  (Variables|Default|SetJump%20Counter (Variables|Default|GetMax%20Jumps))
  (Variables|Default|SetDash%20Counter (Variables|Default|GetMax%20Dashes))
  (Variables|Default|SetbCanAirJump true)
  (Variables|Default|SetbCanAirDash true))

(event Custom|Check%20If%20Out%20of%20Movement
  (if (and (== (Variables|Default|GetJump%20Counter) 0) (== (Variables|Default|GetDash%20Counter) 0))
    (Variables|Default|SetbSelfDestruct true)
    (bind _returnvalue (Utilities|Time|SetTimerbyEvent (delegate Custom|Die) 5.0))
    (Variables|Default|SetSelfDestructTimer _returnvalue)))

(event Custom|Start%20Win
  (Utilities|Time|ClearandInvalidateTimerbyHandle (Variables|Default|GetSelfDestructTimer))
  (Variables|Default|SetbSelfDestruct false)
  (Input|DisableInput (Game|GetPlayerController 0))
  (Development|PrintString "You Did It!!!!!"))

(event EventOnMovementModeChanged
  (params (PrevMovementMode :type EMovementMode%20Enum :default "MOVE_None") (NewMovementMode :type EMovementMode%20Enum :default "MOVE_None") (PrevCustomMode :type Byte :default 0) (NewCustomMode :type Byte :default 0))
  (if (and (Utilities|Enum|Equal(Enum) PrevMovementMode "MOVE_Walking") (Utilities|Enum|Equal(Enum) NewMovementMode "MOVE_Falling"))
    (Variables|Default|SetCoyoteTimeActive true)
    (Utilities|FlowControl|Delay (Variables|Default|GetCoyoteTime))
    (Variables|Default|SetCoyoteTimeActive false)
    (elif (Utilities|Enum|Equal(Enum) NewMovementMode "MOVE_None")
      (Variables|Default|SetbCanAirJump true)
      (Variables|Default|SetbCanAirDash true))))

(event EventTick
  (params (DeltaSeconds :type Float%20%28single-precision%29))
  (bind _returnvalue (Transformation|GetVelocity))
  (Transformation|SetRelativeLocation (Variables|Default|GetSpringArm) (Math|Vector|Lerp(Vector) (Variables|/Script/Engine.SceneComponent|GetRelativeLocation (Variables|Default|GetSpringArm)) (* (Math|Vector|MakeVector 0.0 (CallFunction|SignedSqrt (.y _returnvalue)) (+ (CallFunction|SignedSqrt (.z _returnvalue)) 5e+01)) (Variables|Default|GetCamera%20Lead%20Scale)) (* DeltaSeconds 2.0)) false false))

(event EventBeginPlay
  (bind _returnvalue (UserInterface|CreateWidget "/Game/UI/WBP_CharacterCounters.WBP_CharacterCounters_C" (Game|GetPlayerController 0)))
  (Variables|/Game/UI/WBP_CharacterCounters.WBP_CharacterCounters_C|SetPlayerCharacter _returnvalue self)
  (UserInterface|SetWidget (Variables|Default|GetWidget) _returnvalue)
  (CallFunction|ResetCounters)
  (Variables|Default|SetSpawn%20Location (Transformation|GetActorLocation)))

(event Input|ActionEvents|InputActionJump
  (params (Key :type Key%20Structure :default "None"))
  (bind _sprite (Variables|Default|GetSprite))
  (:Pressed
    (if (CallFunction|CanJump)
      (bind _sprite_scale (Timeline|Jump%20Anim PlayFromStart)
        (:Update
          (Transformation|SetRelativeScale3D _sprite (+ _sprite_scale 1.0))
          (Transformation|SetRelativeLocation _sprite (Math|Vector|MakeVector 0.0 0.0 (- (* (.Z (Math|Vector|BreakVector _sprite_scale)) 5e+01) 5.0)) false false))
        (:Launch
          (CallFunction|CustomJump))))))

(event Input|ActionEvents|InputActionDash
  (params (Key :type Key%20Structure :default "None"))
  (bind _charactermovement (Variables|Character|GetCharacterMovement))
  (:Pressed
    (if (CallFunction|CanDash)
      (Variables|/Script/Engine.CharacterMovementComponent|SetGravityScale (Variables|Character|GetCharacterMovement) 0.0)
      (bind _stretch (Timeline|Dash%20Anim PlayFromStart)
        (:Finished
          (Variables|/Script/Engine.CharacterMovementComponent|SetGravityScale _charactermovement (Math|Float|SelectFloat 0.0 1.0 (Variables|Default|GetbDead)))
          (Components|Movement|StopMovementImmediately _charactermovement)
          (Variables|Default|SetbDashing false))
        (:Func%20Call
          (CallFunction|Dash)
          (Variables|Default|SetbDashing true))))))

(event Input|AxisEvents|InputAxisLateral
  (params (AxisValue :type Float%20%28single-precision%29))
  (Pawn|Input|AddMovementInput (Math|Vector|GetRightVector (Variables|Default|GetCamera)) AxisValue false)
  (Transformation|SetRelativeRotation (Variables|Default|GetSprite) (Math|Rotator|MakeRotator 0.0 0.0 (Math|Float|SelectFloat -9e+01 9e+01 (< AxisValue 0.0))) false false))

(fn ConstructionScript)

(fn CanJump
  (return (and (> (Variables|Default|GetJump%20Counter) 0) (Math|Boolean|ORBoolean (Variables|Default|GetbCanAirJump) (not (AI|Components|NavMovement|IsFalling (Variables|Character|GetCharacterMovement))) (Variables|Default|GetCoyoteTimeActive)))))

(fn CanDash
  (return (and (> (Variables|Default|GetDash%20Counter) 0) (Math|Boolean|ORBoolean (Variables|Default|GetbCanAirDash) (not (AI|Components|NavMovement|IsFalling (Variables|Character|GetCharacterMovement))) (Variables|Default|GetCoyoteTimeActive)))))

(fn SignedSqrt
  (params (Input :type Float%20%28single-precision%29))
  (return (* (Math|Float|Sign(Float) Input) (Math|Float|Sqrt (Math|Float|Absolute(Float) Input)))))